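; Paper2D samurai duelist for a reaction-timing duel driven by GM_Duel, sliding in on BeginPlay and on reset.
; Attack accepts one press per round: during Wait it shows a cross as an early-press penalty, during Draw it ends the game and lunges.
; The attack timeline swaps the sprite mid-lunge and reports success to the game mode.
; It also handles the defeated sprite and tracks losses and win streaks.
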(event Custom|SlideIn
  (Components|Timeline|SetPlayRate (Variables|Default|GetSlideInAnim) 3.0)
  (bind _alpha (Timeline|SlideInAnim PlayFromStart)
    (:Update
      (Transformation|SetRelativeLocation (Variables|Default|GetPaperSprite) (Math|Vector|Lerp(Vector) (Variables|Default|GetSlide%20Start%20Pos) (Variables|Default|GetSprite%20Default%20Pos) _alpha) false false))))

(event Custom|Attack
  (if (not (Variables|Default|GetPressedDraw))
    (switch Utilities|FlowControl|Switch|SwitchonE_Phase (Variables|/Game/Dynamic/Blueprints/GM_Duel.GM_Duel_C|GetPhase (Variables|Default|GetGamemode))
      (:NewEnumerator1
        (CallFunction|SetCrossVisibility true)
        (Variables|Default|SetPressedDraw true))
      (:NewEnumerator2
        (Variables|Default|SetPressedDraw true)
        (Default|SetGameFinished (Variables|Default|GetGamemode))
        (Components|Timeline|SetPlayRate (Variables|Default|GetAttackAnim) 8.0)
        (bind _alpha (Timeline|AttackAnim PlayFromStart)
          (:Update
            (Transformation|SetRelativeLocation (Variables|Default|GetPaperSprite) (Math|Vector|Lerp(Vector) (Variables|Default|GetSprite%20Default%20Pos) (Variables|/Script/Engine.SceneComponent|GetRelativeLocation (Variables|Default|GetAttackPos)) _alpha) false false))
          (:SwitchSprite
            (CallFunction|UpdateSprite (Variables|Default|GetAttackSprite))
            (Default|AttackedSuccessfully (Variables|Default|GetGamemode) (Pawn|IsPlayerControlled))))))))

(event Custom|Defeated
  (Rendering|Components|Sprite|SetSprite (Variables|Default|GetPaperSprite) (Variables|Default|GetDefeatedSprite))
  (CallFunction|SetCrossVisibility false))

(event EventBeginPlay
  (bind _asgm_duel (Utilities|Casting|CastToGM_Duel (Game|GetGameMode)))
  (Variables|Default|SetGamemode _asgm_duel)
  (Variables|Default|SetSprite%20Default%20Pos (Variables|/Script/Engine.SceneComponent|GetRelativeLocation (Variables|Default|GetPaperSprite)))
  (CallFunction|Slidein)
  (CallFunction|SetCrossVisibility false))

(event Collision|EventActorBeginOverlap
  (params (OtherActor :type Actor%20Object%20Reference)))

(event EventTick
  (params (DeltaSeconds :type Float%20%28single-precision%29)))

(fn ConstructionScript)

(fn SetCrossVisibility
  (params (bNewVisibility :type Boolean))
  (Rendering|SetVisibility (Variables|Default|GetCross) bNewVisibility false))

(fn UpdateSprite
  (params (NewSprite :type Paper%20Sprite%20Object%20Reference))
  (Rendering|Components|Sprite|SetSprite (Variables|Default|GetPaperSprite) NewSprite)
  (Rendering|Material|SetMaterial (Variables|Default|GetPaperSprite) 0 "/Paper2D/TranslucentUnlitSpriteMaterial.TranslucentUnlitSpriteMaterial")
  (Rendering|SetTranslucentSortPriority (Variables|Default|GetPaperSprite) 1))

(fn Reset
  (Rendering|Components|Sprite|SetSprite (Variables|Default|GetPaperSprite) (Variables|Default|GetIdleSprite))
  (Variables|Default|SetPressedDraw false)
  (CallFunction|Slidein))

(fn RecordWin
  (Variables|Default|SetWinStreak (+ (Variables|Default|GetWinStreak) 1))
  (if (> (+ (Variables|Default|GetWinStreak) 1) (Variables|Default|GetMaxWinStreak))
    (bind _output_get (Variables|Default|SetMaxWinStreak (+ (Variables|Default|GetWinStreak) 1)))))

(fn RecordLoss
  (Variables|Default|SetLosses (+ (Variables|Default|GetLosses) 1))
  (Variables|Default|SetWinStreak 0))